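; BP_MyChar is a character Blueprint that equips itself with attached hit-part and weapon actors when play begins.
; BeginPlay attaches a spawned BP_BareHands to head, hand and leg sockets on the mesh, plus BP_Axe_Weapon when kusaGameInstance's CharNumberIndex selects that character.
; Debug keys set BisDead (J) and print attached actor names (K).
; Unconnected leftover nodes hold jump, velocity and health-print logic that never runs.
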(event `self.ReceiveBeginPlay`
  ;[1 1 1] HeadSpawn
  (bind _returnvalue (`|SpawnActorFromClass` "/Game/BluePrints/weapons/BP_BareHands.BP_BareHands_C" (`KismetMathLibrary.MakeTransform` (0.0 0.0 0.0)) "AlwaysSpawn" "OverrideRootScale" null null))
  (`self.K2_AttachToComponent` _returnvalue (`self.Mesh`) "HeadSocket" "SnapToTarget" "SnapToTarget" "SnapToTarget" true)
  ;[1 1 1] LefthandSpawn
  (bind _returnvalue_2 (`|SpawnActorFromClass` "/Game/BluePrints/weapons/BP_BareHands.BP_BareHands_C" (`KismetMathLibrary.MakeTransform` (0.0 0.0 0.0)) "AlwaysSpawn" "OverrideRootScale" null null))
  (`self.K2_AttachToComponent` _returnvalue_2 (`self.Mesh`) "S_Char1_LeftHand" "SnapToTarget" "SnapToTarget" "SnapToTarget" true)
  ;[1 1 1] RighthandSpawn
  (bind _returnvalue_3 (`|SpawnActorFromClass` "/Game/BluePrints/weapons/BP_BareHands.BP_BareHands_C" (`KismetMathLibrary.MakeTransform` (0.0 0.0 0.0)) "AlwaysSpawn" "OverrideRootScale" null null))
  (`self.K2_AttachToComponent` _returnvalue_3 (`self.Mesh`) "S_Char1_RightHand" "SnapToTarget" "SnapToTarget" "SnapToTarget" true)
  ;[1 1 1] LeftLegSpawn
  (bind _returnvalue_4 (`|SpawnActorFromClass` "/Game/BluePrints/weapons/BP_BareHands.BP_BareHands_C" (`KismetMathLibrary.MakeTransform` (0.0 0.0 0.0)) "AlwaysSpawn" "OverrideRootScale" null null))
  (`self.K2_AttachToComponent` _returnvalue_4 (`self.Mesh`) "S_Char1_LeftLeg" "SnapToTarget" "SnapToTarget" "SnapToTarget" true)
  ;[1 1 1] RightLegSpawn
  (bind _returnvalue_5 (`|SpawnActorFromClass` "/Game/BluePrints/weapons/BP_BareHands.BP_BareHands_C" (`KismetMathLibrary.MakeTransform` (0.0 0.0 0.0)) "AlwaysSpawn" "OverrideRootScale" null null))
  (`self.K2_AttachToComponent` _returnvalue_5 (`self.Mesh`) "S_Char1_RightLeg" "SnapToTarget" "SnapToTarget" "SnapToTarget" true)
  (bind _askusa_game_instance (cast `kusaGameInstance` (`GameplayStatics.GetGameInstance`)))
  (if (== (`kusaGameInstance.CharNumberIndex` _askusa_game_instance) 2)
    ;[1 1 1] AxeSpawn
    (bind _returnvalue_6 (`|SpawnActorFromClass` "/Game/BluePrints/weapons/BP_Axe_Weapon.BP_Axe_Weapon_C" (`KismetMathLibrary.MakeTransform` (0.0 0.0 0.0)) "AlwaysSpawn" "OverrideRootScale" null null))
    (`self.K2_AttachToComponent` _returnvalue_6 (`self.Mesh`) "ForAxe" "SnapToTarget" "SnapToTarget" "SnapToTarget" true))
  (set `self.TempRet` 5))

(event `Key|J`
  (params (Key :type "Key Structure"))
  (:`Pressed`
    (set `self.bisDead` true)))

(event `Key|K`
  (params (Key :type "Key Structure"))
  (:`Pressed`
    (for _array_element (`self.GetAttachedActors` true)
      (`KismetSystemLibrary.PrintString` (`KismetSystemLibrary.GetDisplayName` _array_element) true true (struct :`G` 0.66 :`B` 1.0 :`A` 1.0) 0.0))))

(event `self.ReceiveTick`
  (params (DeltaSeconds :type "Float (single-precision)")))

(fn `UserConstructionScript`)