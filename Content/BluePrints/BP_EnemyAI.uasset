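; BP_EnemyAI is an enemy actor that can spawn armed with an axe, though it holds no AI decision logic itself.
; On BeginPlay it reads EnemyNumberIndex from kusaGameInstance and, if it equals 2, spawns a BP_Axe_Weapon snapped to the ForAxe socket on its Mesh.
; Every Tick it sets the BisEnemy flag and prints Health on screen as debug output.
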(event `self.ReceiveBeginPlay`
  (bind _askusa_game_instance (cast `kusaGameInstance` (`GameplayStatics.GetGameInstance`)))
  (if (== (`kusaGameInstance.EnemyNumberIndex` _askusa_game_instance) 2)
    ;[1 1 1] AxeSpawn
    (bind _returnvalue (`|SpawnActorFromClass` "/Game/BluePrints/weapons/BP_Axe_Weapon.BP_Axe_Weapon_C" (`KismetMathLibrary.MakeTransform` (0.0 0.0 0.0)) "AlwaysSpawn" "OverrideRootScale" null null))
    (`self.K2_AttachToComponent` _returnvalue (`self.Mesh`) "ForAxe" "SnapToTarget" "SnapToTarget" "SnapToTarget" true)))

(event `self.ReceiveTick`
  (params (DeltaSeconds :type "Float (single-precision)"))
  (set `self.bisEnemy` true)
  (`KismetSystemLibrary.PrintString` (`KismetStringLibrary.Conv_DoubleToString` (`self.Health`)) true true (struct :`R` 0.066051 :`G` 1.0 :`A` 1.0) 0.0))

(fn `UserConstructionScript`)